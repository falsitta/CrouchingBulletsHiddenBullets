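; TestWallBP is a destructible wall that breaks when a downed ThirdPersonCharacter hits it.
; On hit, it applies radius damage and an impulse to its Destructible, scaled from the ragdoll's pelvis velocity plus the character's stored velocity values, and spawns an impact particle effect.
; Walls flagged as the final barrier react only when the character's Multiplier is above a high threshold.
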(event `self.ReceiveHit`
  (params (MyComp :type "PrimitiveComponent Object Reference") (Other :type "Actor Object Reference") (OtherComp :type "PrimitiveComponent Object Reference") (bSelfMoved :type Boolean) (HitLocation :type "Vector Structure") (HitNormal :type "Vector Structure") (NormalImpulse :type "Vector Structure") (Hit :type "HitResult Structure (by ref)"))
  (bind _destructible (`self.Destructible`))
  (bind _asthird_person_character (cast `/Game/ThirdPersonBP/Blueprints/ThirdPersonCharacter` Other))
  (if (`/Game/ThirdPersonBP/Blueprints/ThirdPersonCharacter.Down` _asthird_person_character)
    (if (`self.Finalbarier`)
      (if (> (`/Game/ThirdPersonBP/Blueprints/ThirdPersonCharacter.Multiplier` _asthird_person_character) 90.0)
        (bind _returnvalue (`PrimitiveComponent.GetPhysicsLinearVelocity` (`Character.Mesh` _asthird_person_character) "pelvis" :!label _label))
        (`DestructibleComponent.ApplyRadiusDamage` _destructible (+ (`KismetMathLibrary.VSize` _returnvalue) (`/Game/ThirdPersonBP/Blueprints/ThirdPersonCharacter.Velocity` _asthird_person_character)) HitLocation 150.0 2.0 false)
        (`PrimitiveComponent.AddImpulseAtLocation` _destructible (* (+ _returnvalue (`/Game/ThirdPersonBP/Blueprints/ThirdPersonCharacter.VelVect` _asthird_person_character)) 3.0) HitLocation "None")
        (`GameplayStatics.SpawnEmitterAtLocation` "/Game/MatrixSymbols/MatrixImpact.MatrixImpact" HitLocation (`KismetMathLibrary.Conv_VectorToRotator` HitNormal)))
      (else
        (goto _label)))))

(fn `UserConstructionScript`)